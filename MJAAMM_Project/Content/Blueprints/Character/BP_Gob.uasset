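; BP_Gob is a character Blueprint that implements the Gob's frame-triggered special moves, Arrow and Slide.
; Arrow spawns a scaled-down arrow projectile at a spawn point on a set animation frame.
; Slide uses a timeline to drive forward velocity with a gravity-based downward component, and getting hit during it stops the timeline.
; Normal move handlers are empty stubs, and debug prints remain.
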(event `self.Normal_Move_Event`
  (params (Normal :type "/Game/Blueprints/Character/E_Normal_Move Enum" :default "NewEnumerator1") (Frame :type Integer))
  (switch `/Game/Blueprints/Character/E_Normal_Move` Normal))

(event `Spawn_Arrow`
  (bind (_returnvalue_location _returnvalue_rotation) (`KismetMathLibrary.BreakTransform` (`SceneComponent.K2_GetComponentToWorld` (`self.Arrow_SpawnPoint1`))))
  (bind _returnvalue (`|SpawnActorFromClass` "/Game/Blueprints/Character/Chara_Gob/Projectile/BP_Projectile_Arrow.BP_Projectile_Arrow_C" (`KismetMathLibrary.MakeTransform` _returnvalue_location _returnvalue_rotation (0.25 0.25 0.25)) "AlwaysSpawn" "OverrideRootScale" null null))
  (`KismetSystemLibrary.PrintString` (`KismetSystemLibrary.GetDisplayName` _returnvalue)))

(event `self.Special_Move_Event`
  (params (Special :type Name) (Frame :type Integer))
  (switch `name` Special
    (:`Arrow`
      (switch `int` Frame
        (:`13`
          (`self.Spawn_Arrow`))))
    (:`Slide`
      (switch `int` Frame
        (:`16`
          (`TimelineComponent.SetPlayRate` (`self.Timeline_Slide`) (/ 1.0 (`self.Slide_Duration`)))
          (`KismetSystemLibrary.PrintString` "Start Slide")
          (bind (_direction _newtrack_0) (`Timeline|Timeline_Slide` :!via `PlayFromStart` :!label _label)
            (:`Update`
              (set `MovementComponent.Velocity` (+ (* (`KismetMathLibrary.Vector_Down`) (* (`MovementComponent.GetGravityZ` (`self.CharacterMovement`)) -1.0)) (* (`self.GetActorForwardVector`) (* _newtrack_0 (`self.Slide_Strength`)))) (`self.CharacterMovement`)))
            (:`Finished`
              (`KismetSystemLibrary.PrintString` "Stop Slide"))))))))

(event `Stop_Slide`
  (goto _label :!via `Stop`))

(event `self.OnHit`
  (params (ActorHit :type "Actor Object Reference"))
  (switch `/Game/Blueprints/Character/E_State_Combat` (`self.Current_State_Combat`)
    (:`NewEnumerator2`
      (switch `name` (`self.Current_Special`)
        (:`Slide`
          (`self.Stop_Slide`))))
    (:`NewEnumerator1`
      (switch `/Game/Blueprints/Character/E_Normal_Move` (`self.Current_Normal`)))))

(fn `UserConstructionScript`
  (`parent.UserConstructionScript`))