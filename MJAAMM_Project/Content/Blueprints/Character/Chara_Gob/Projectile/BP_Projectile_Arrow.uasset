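; BP_Projectile_Arrow is an arrow projectile built on a paper sprite.
; On BeginPlay it caches the BP_PlayerCharacter in the level and destroys itself after five seconds.
; When the sprite overlaps any actor other than that player, it prints a debug hit message with the actor's name and destroys itself immediately, applying no damage.
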(event `self.ReceiveBeginPlay`
  (bind _returnvalue (`GameplayStatics.GetActorOfClass` "/Game/Blueprints/Character/BP_PlayerCharacter.BP_PlayerCharacter_C"))
  (set `self.Chara` _returnvalue)
  (`KismetSystemLibrary.Delay` 5.0)
  (`self.K2_DestroyActor` :!label _label))

(event `self.PaperSprite.OnComponentBeginOverlap`
  (params (OverlappedComponent :type "PrimitiveComponent Object Reference") (OtherActor :type "Actor Object Reference") (OtherComp :type "PrimitiveComponent Object Reference") (OtherBodyIndex :type Integer) (bFromSweep :type Boolean) (SweepResult :type "HitResult Structure (by ref)"))
  (if (!= OtherActor (`self.Chara`))
    (`KismetSystemLibrary.PrintString` (`KismetStringLibrary.Concat_StrStr` "ARROW HAS HIT           " (`KismetSystemLibrary.GetDisplayName` OtherActor)) true true (struct :`R` 0.001163 :`G` 0.4375 :`A` 1.0))
    (goto _label)))

(fn `UserConstructionScript`)