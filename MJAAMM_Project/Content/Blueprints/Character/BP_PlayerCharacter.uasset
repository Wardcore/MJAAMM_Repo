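; Base 2D fighting-game character on Paper2D flipbooks, driven by a CharaData asset for movement, normals and specials.
; Axis and Punch/Kick inputs drive movement, stance-based normals and a 30-entry per-tick buffer, scanned backwards for special sequences.
; Flipbook frames set Startup/Hit/Recovery, toggling sprite collision for overlap hits; normals that hit can cancel during recovery.
; Move, hit and rotation events are empty hooks; Tick prints debug state.
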(event `InputAction|Up`
  (params (Key :type "Key Structure"))
  ;[1 1 1] Comment
)

(event `InputAction|Down`
  (params (Key :type "Key Structure"))
  ;[1 1 1] Comment
)

(event `InputAction|Right`
  (params (Key :type "Key Structure"))
  ;[1 1 1] Comment
)

(event `InputAction|Left`
  (params (Key :type "Key Structure"))
  ;[1 1 1] Comment
)

(event `self.ReceiveBeginPlay`
  (bind _chara_data (`self.Chara_Data`))
  (`self.Chara_Data`
    (:`then`
      (`PrimitiveComponent.SetCollisionEnabled` (`self.Sprite`) "NoCollision")
      (set `/Game/Blueprints/Components/Comp_Health.Health` (`/Game/Blueprints/Character/PDA_Chara.HealthPool` _chara_data) (`self.Comp_Health`))
      (set `CharacterMovementComponent.MaxWalkSpeed` (`/Game/Blueprints/Character/PDA_Chara.Speed_walk` _chara_data) (`self.CharacterMovement`)))
    (:`else`
      (`KismetSystemLibrary.PrintString` "ERROR DATA NOT VALID" true true (struct :`R` 1.0 :`A` 1.0)))))

(event `InputAxis|Right_Left_Axis`
  (params (AxisValue :type "Float (single-precision)"))
  (bind (_stick_axes_x _stick_axes_y) (`KismetMathLibrary.BreakVector2D` (`self.Stick_axes`)))
  (bind _output_get (set `self.Stick_axes` (`KismetMathLibrary.MakeVector2D` AxisValue _stick_axes_y)))
  (setmembers `/Game/Blueprints/Character/Inputs/Struct_Buffer_Data` :`StructRef` (`self.Input_CurrentFrame`) :`Direction` (`self.AxisValueToInput` _output_get))
  (switch `/Game/Blueprints/Character/E_State_MVT` (`self.Current_State_MVT`)
    (:`NewEnumerator0`
      _)
    (:`NewEnumerator1`
      _)
    (:`NewEnumerator4`
      _)
    (:`NewEnumerator2`
      _))
  (switch `/Game/Blueprints/Character/E_State_Combat` (`self.Current_State_Combat`)
    (:`NewEnumerator0`
      (`self.AddMovementInput` (1.0 0.0 0.0) AxisValue))))

(event `InputAxis|Up_Down_Axis`
  (params (AxisValue :type "Float (single-precision)"))
  (bind _stick_axes_x (`KismetMathLibrary.BreakVector2D` (`self.Stick_axes`)))
  (bind _output_get (set `self.Stick_axes` (`KismetMathLibrary.MakeVector2D` _stick_axes_x AxisValue)))
  (setmembers `/Game/Blueprints/Character/Inputs/Struct_Buffer_Data` :`StructRef` (`self.Input_CurrentFrame`) :`Direction` (`self.AxisValueToInput` _output_get))
  (`self.Compare to Dead Zone` AxisValue
    (:`>=`
      (`self.UnCrouch`)
      (switch `/Game/Blueprints/Character/E_State_MVT` (`self.Current_State_MVT`)
        (:`NewEnumerator0`
          _)
        (:`NewEnumerator1`
          _)
        (:`NewEnumerator4`
          _)
        (:`NewEnumerator3`
          _))
      (switch `/Game/Blueprints/Character/E_State_Combat` (`self.Current_State_Combat`)
        (:`NewEnumerator0`
          (`self.Jump`))))
    (:`between`
      (`self.UnCrouch`)
      (`self.StopJumping`))
    (:`<=`
      (`self.StopJumping`)
      (switch `/Game/Blueprints/Character/E_State_MVT` (`self.Current_State_MVT`)
        (:`NewEnumerator0`
          _)
        (:`NewEnumerator1`
          _)
        (:`NewEnumerator4`
          _)
        (:`NewEnumerator3`
          _))
      (switch `/Game/Blueprints/Character/E_State_Combat` (`self.Current_State_Combat`)
        (:`NewEnumerator0`
          (`self.Crouch`))))))

(event `InputAction|Run`
  (params (Key :type "Key Structure")))

(event `self.ReceiveTick`
  (params (DeltaSeconds :type "Float (single-precision)"))
  (bind _sprite (`self.Sprite`))
  (bind _current_state_frame (`self.Current_State_Frame`))
  (bind _sprite_2 (`self.Sprite`))
  (bind _returnvalue (`PaperFlipbookComponent.GetPlaybackPositionInFrames` (`self.Sprite`)))
  (bind (_relativelocation_x _relativelocation_y) (`KismetMathLibrary.BreakVector` (`SceneComponent.RelativeLocation` _sprite)))
  (`|ExecutionSequence`
    (:`then_0`
      (`|ExecutionSequence`
        (:`then_0`
          (`|ExecutionSequence`
            (:`then_0`
              (`self.Record Input Buffer`)
              (`self.CheckInputBufferForSpecial`))
            (:`then_1`
              (`self.UpdateAttackState`))))
        (:`then_1`
          (`|ExecutionSequence`
            (:`then_0`
              (`self.Check_Ground`))
            (:`then_1`
              (`self.Update_Movement_State`)
              (`self.Update_MVT_Animation`))
            (:`then_2`
              (`self.UpdateRotation`))))
        (:`then_4`
          (`SceneComponent.K2_SetRelativeLocation` _sprite (`KismetMathLibrary.MakeVector` _relativelocation_x _relativelocation_y (* (`CapsuleComponent.CapsuleHalfHeight` (`self.CapsuleComponent`)) -1.0)) false false)
          (if (`SceneComponent.DoesSocketExist` _sprite_2 "Head")
            (`SceneComponent.K2_SetWorldLocation` (`self.SpriteHead`) (`SceneComponent.GetSocketLocation` _sprite_2 "Head") false false)
            (else
              (`KismetSystemLibrary.PrintString` (`KismetStringLibrary.Concat_StrStr` "ERROR NO HEAD SOCKET IN    " (`KismetSystemLibrary.GetDisplayName` (`PaperFlipbook.GetSpriteAtFrame` (`PaperFlipbookComponent.GetFlipbook` _sprite_2) (`PaperFlipbookComponent.GetPlaybackPositionInFrames` _sprite_2)))) true true (struct :`R` 1.0 :`A` 1.0) 0.5))))))
    (:`then_1`
      (if true
        (`|ExecutionSequence`
          (:`then_0`
            (`KismetSystemLibrary.PrintString` "-----------------------------------" true false (struct :`R` 1.0 :`G` 1.0 :`B` 1.0 :`A` 1.0) 0.0)
            (`KismetSystemLibrary.PrintString` (`KismetStringLibrary.Concat_StrStr` "MVT:    " (`|GetEnumeratorNameAsString` (`self.Current_State_MVT`)) "    Velocity:         " (`KismetStringLibrary.Conv_DoubleToString` (`KismetMathLibrary.VSize` (`MovementComponent.Velocity` (`self.CharacterMovement`))))) true false (struct :`G` 0.66 :`B` 1.0 :`A` 1.0) 0.0)
            (`KismetSystemLibrary.PrintString` (`KismetStringLibrary.Concat_StrStr` "MOVES:   " (`|GetEnumeratorNameAsString` (`self.Current_Normal`)) "   " (`KismetStringLibrary.Conv_IntToString` (select `/Game/Blueprints/Character/E_State_MoveFrame` _current_state_frame :`NewEnumerator0` _returnvalue :`NewEnumerator1` _returnvalue :`NewEnumerator2` _returnvalue)) "   " (`|GetEnumeratorNameAsString` _current_state_frame)) true false (select `/Game/Blueprints/Character/E_State_MoveFrame` _current_state_frame :`NewEnumerator3` (struct :`R` 1.0 :`G` 1.0 :`B` 1.0 :`A` 1.0) :`NewEnumerator0` (struct :`G` 0.16237 :`B` 1.0 :`A` 1.0) :`NewEnumerator1` (struct :`R` 1.0 :`G` 0.026519 :`A` 1.0) :`NewEnumerator2` (struct :`R` 1.0 :`G` 0.853839 :`A` 1.0) :!type "LinearColor Structure") 0.0)
            (`KismetSystemLibrary.PrintString` "-----------------------------------" true false (struct :`R` 1.0 :`G` 1.0 :`B` 1.0 :`A` 1.0) 0.0)))))))

(event `InputAction|Punch`
  (params (Key :type "Key Structure"))
  (bind _input_currentframe (`self.Input_CurrentFrame`))
  (bind (_normals_punch_neutral _normals_punch_low _normals_punch_air _normals_kick_neutral _normals_kick_low _normals_kick_air) (break `/Game/Blueprints/Character/F_List_Normals` (`/Game/Blueprints/Character/PDA_Chara.Normals` (`self.Chara_Data`))))
  (bind (_move_special _move_normal _inputs _flipbook) (break `/Game/Blueprints/Character/F_info_Move` _normals_punch_neutral))
  (bind (_move_special_2 _move_normal_2 _inputs_2 _flipbook_2) (break `/Game/Blueprints/Character/F_info_Move` _normals_punch_air))
  (bind (_move_special_3 _move_normal_3 _inputs_3 _flipbook_3) (break `/Game/Blueprints/Character/F_info_Move` _normals_punch_low))
  (:`Pressed`
    (setmembers `/Game/Blueprints/Character/Inputs/Struct_Buffer_Data` :`StructRef` _input_currentframe :`Punch` true)
    (switch `/Game/Blueprints/Character/E_State_MVT` (`self.Current_State_MVT`)
      (:`NewEnumerator0`
        (`self.CanCancelFrom` :!label _label)
        (`self.Play_Move` "NewEnumerator1" _move_special _move_normal _flipbook))
      (:`NewEnumerator1`
        (goto _label))
      (:`NewEnumerator4`
        (goto _label))
      (:`NewEnumerator3`
        (`self.CanCancelFrom`)
        (`self.Play_Move` "NewEnumerator1" _move_special_3 _move_normal_3 _flipbook_3))
      (:`NewEnumerator2`
        (`self.CanCancelFrom`)
        (`self.Play_Move` "NewEnumerator1" _move_special_2 _move_normal_2 _flipbook_2))))
  (:`Released`
    (setmembers `/Game/Blueprints/Character/Inputs/Struct_Buffer_Data` :`StructRef` _input_currentframe :`Punch` false)))

(event `Play_Move`
  (params (CombatState :type "/Game/Blueprints/Character/E_State_Combat Enum" :default "NewEnumerator1") (Move_Special :type Name) (Move_Normal :type "/Game/Blueprints/Character/E_Normal_Move Enum" :default "NewEnumerator0") (Move_Flipbook :type "PaperFlipbook Object Reference"))
  (bind _sprite (`self.Sprite`))
  (bind _output_get (set `self.Current_State_Combat` CombatState))
  (switch `/Game/Blueprints/Character/E_State_Combat` _output_get
    (:`NewEnumerator0`
      (`KismetSystemLibrary.PrintString` "ERROR move during neutral combat state" true true (struct :`R` 1.0 :`A` 1.0)))
    (:`NewEnumerator2`
      (set `self.Current_Special` Move_Special)
      (`PaperFlipbookComponent.SetFlipbook` _sprite Move_Flipbook :!label _label_2)
      (`PaperFlipbookComponent.PlayFromStart` _sprite)
      (`KismetSystemLibrary.RetriggerableDelay` (`PaperFlipbookComponent.GetFlipbookLength` _sprite))
      (set `self.Current_State_Combat` "NewEnumerator0")
      (`KismetSystemLibrary.PrintString` "END OF MOVE !" false false (struct :`R` 0.722252 :`B` 1.0 :`A` 1.0) 1.0)
      (set `self.hasHit` false))
    (:`NewEnumerator1`
      (set `self.Current_Normal` Move_Normal)
      (goto _label_2))))

(event `InputAction|Kick`
  (params (Key :type "Key Structure"))
  (bind _input_currentframe (`self.Input_CurrentFrame`))
  (bind (_normals_punch_neutral _normals_punch_low _normals_punch_air _normals_kick_neutral _normals_kick_low _normals_kick_air) (break `/Game/Blueprints/Character/F_List_Normals` (`/Game/Blueprints/Character/PDA_Chara.Normals` (`self.Chara_Data`))))
  (bind (_move_special _move_normal _inputs _flipbook) (break `/Game/Blueprints/Character/F_info_Move` _normals_kick_low))
  (bind (_move_special_2 _move_normal_2 _inputs_2 _flipbook_2) (break `/Game/Blueprints/Character/F_info_Move` _normals_kick_neutral))
  (bind (_move_special_3 _move_normal_3 _inputs_3 _flipbook_3) (break `/Game/Blueprints/Character/F_info_Move` _normals_kick_air))
  (:`Pressed`
    (setmembers `/Game/Blueprints/Character/Inputs/Struct_Buffer_Data` :`StructRef` _input_currentframe :`Kick` true)
    (switch `/Game/Blueprints/Character/E_State_MVT` (`self.Current_State_MVT`)
      (:`NewEnumerator0`
        (`self.CanCancelFrom` :!label _label_3)
        (`self.Play_Move` "NewEnumerator1" _move_special_2 _move_normal_2 _flipbook_2))
      (:`NewEnumerator1`
        (goto _label_3))
      (:`NewEnumerator4`
        (goto _label_3))
      (:`NewEnumerator3`
        (`self.CanCancelFrom`)
        (`self.Play_Move` "NewEnumerator1" _move_special _move_normal _flipbook))
      (:`NewEnumerator2`
        (`self.CanCancelFrom`)
        (`self.Play_Move` "NewEnumerator1" _move_special_3 _move_normal_3 _flipbook_3))))
  (:`Released`
    (setmembers `/Game/Blueprints/Character/Inputs/Struct_Buffer_Data` :`StructRef` _input_currentframe :`Kick` false)))

(event `PlaySpecialMove`
  (params (SpecialMove :type "/Game/Blueprints/Character/F_info_Move Structure"))
  (bind (_move_special _move_normal _inputs _flipbook) (break `/Game/Blueprints/Character/F_info_Move` SpecialMove))
  (`self.CanCancelFrom`)
  (`self.Play_Move` "NewEnumerator2" _move_special _move_normal _flipbook))

(event `Update_Movement_State`
  (bind _returnvalue (`KismetMathLibrary.VSize` (`MovementComponent.Velocity` (`self.CharacterMovement`))))
  (if (`self.bIsCrouched`)
    (set `self.Current_State_MVT` "NewEnumerator3")
    (elif (not (`self.isGrounded`))
      (set `self.Current_State_MVT` "NewEnumerator2")
      (elif (> _returnvalue 0.0)
        (if (> _returnvalue 300.0)
          (set `self.Current_State_MVT` "NewEnumerator4")
          (else
            (set `self.Current_State_MVT` "NewEnumerator1")))
        (else
          (set `self.Current_State_MVT` "NewEnumerator0"))))))

(event `Check_Ground`
  (bind _returnvalue (`self.K2_GetActorLocation`))
  (bind _returnvalue_2 (`CapsuleComponent.GetScaledCapsuleRadius` (`self.CapsuleComponent`)))
  (bind (_outhit _returnvalue_3) (`KismetSystemLibrary.CapsuleTraceSingle` _returnvalue (+ _returnvalue (* (`self.GetActorUpVector`) (* (+ (`CapsuleComponent.CapsuleHalfHeight` (`self.CapsuleComponent`)) 10.0) -1.0))) _returnvalue_2 _returnvalue_2 "TraceTypeQuery1"))
  (set `self.isGrounded` _returnvalue_3))

(event `Special_Move_Event`
  (params (Special :type Name) (Frame :type Integer)))

(event `Normal_Move_Event`
  (params (Normal :type "/Game/Blueprints/Character/E_Normal_Move Enum" :default "NewEnumerator1") (Frame :type Integer)))

(event `Update_MVT_Animation`
  (bind (_movement_idle _movement_walk _movement_run _movement_crouch _movement_jump) (break `/Game/Blueprints/Character/F_List_MVT` (`/Game/Blueprints/Character/PDA_Chara.Movement` (`self.Chara_Data`))))
  (if (`|EnumEquality` (`self.Current_State_Combat`) "NewEnumerator0")
    (`PaperFlipbookComponent.SetFlipbook` (`self.Sprite`) (select `/Game/Blueprints/Character/E_State_MVT` (`self.Current_State_MVT`) :`NewEnumerator0` _movement_idle :`NewEnumerator1` _movement_walk :`NewEnumerator4` _movement_run :`NewEnumerator3` _movement_crouch :`NewEnumerator2` _movement_jump))))

(event `UpdateRotation`)

(event `OnHit`
  (params (ActorHit :type "Actor Object Reference")))

(event `UpdateAttackState`
  (bind _sprite (`self.Sprite`))
  (bind _current_state_frame (`self.Current_State_Frame`))
  (bind (_move_special _move_normal _inputs _flipbook _frames_startup _frames_hit _frames_recovery) (break `/Game/Blueprints/Character/F_info_Move` (`self.GetCurrentSpecialData_FromName` (`self.Current_Special`))))
  (bind (_move_special_2 _move_normal_2 _inputs_2 _flipbook_2 _frames_startup_2 _frames_hit_2 _frames_recovery_2) (break `/Game/Blueprints/Character/F_info_Move` (`self.GetCurrentNormalData` (`self.Current_Normal`))))
  (`|ExecutionSequence`
    (:`then_0`
      (switch `/Game/Blueprints/Character/E_State_Combat` (`self.Current_State_Combat`)
        (:`NewEnumerator0`
          (set `self.Current_State_Frame` "NewEnumerator3"))
        (:`NewEnumerator2`
          (`self.SetAttackStateWithFrames` _frames_startup _frames_hit _frames_recovery)
          (bind _current_frame (`self.Tick_Frame_by_Frame`))
          (`self.Special_Move_Event` _move_special _current_frame))
        (:`NewEnumerator1`
          (`self.SetAttackStateWithFrames` _frames_startup_2 _frames_hit_2 _frames_recovery_2)
          (bind _current_frame_2 (`self.Tick_Frame_by_Frame`))
          (`self.Normal_Move_Event` _move_normal_2 _current_frame_2))))
    (:`then_1`
      (if (`|EnumInequality` (`self.OLD_State_Frame`) (`self.Current_State_Frame`))
        (bind _output_get (set `self.OLD_State_Frame` _current_state_frame))
        (`self.OnAttackStateChange` _current_state_frame)
        (switch `/Game/Blueprints/Character/E_State_MoveFrame` _output_get
          (:`NewEnumerator1`
            (`PrimitiveComponent.SetCollisionEnabled` _sprite "QueryAndPhysics"))
          (:`NewEnumerator2`
            (`PrimitiveComponent.SetCollisionEnabled` _sprite "NoCollision")))))
    (:`then_2`
      (switch `/Game/Blueprints/Character/E_State_MoveFrame` (`self.Current_State_Frame`)))))

(event `self.Sprite.OnComponentBeginOverlap`
  (params (OverlappedComponent :type "PrimitiveComponent Object Reference") (OtherActor :type "Actor Object Reference") (OtherComp :type "PrimitiveComponent Object Reference") (OtherBodyIndex :type Integer) (bFromSweep :type Boolean) (SweepResult :type "HitResult Structure (by ref)"))
  (if (!= OtherActor self)
    (`/Engine/EditorBlueprintResources/StandardMacros.IsValid` (`self.GetComponentByClass` OtherActor "/Game/Blueprints/Components/Comp_Health.Comp_Health_C")
      (:`Is Valid`
        (`KismetSystemLibrary.PrintString` (`KismetStringLibrary.Concat_StrStr` "Hit   " (`KismetSystemLibrary.GetDisplayName` OtherActor) "    in     " (`KismetSystemLibrary.GetDisplayName` OtherComp)) true true (struct :`R` 1.0 :`B` 0.543095 :`A` 1.0) 0.5)
        (set `self.hasHit` true)
        (bind _output_get (set `self.ActorHit` OtherActor))
        (`self.OnHit` _output_get)
        (`PrimitiveComponent.SetCollisionEnabled` (`self.Sprite`) "NoCollision")
        (`|ExecutionSequence`)))))

(fn `AxisValueToInput`
  (params (Stick_Axes :type "Vector2D Structure"))
  (returns (out_Dir :type "/Game/Blueprints/Character/Inputs/E_Input_List Enum"))
  (locals (Stick_Dir_Temp :type "/Game/Blueprints/Character/Inputs/E_Input_List Enum"))
  (`|ExecutionSequence`
    (:`then_0`
      (`self.Compare to Dead Zone` (`.Y` (`KismetMathLibrary.BreakVector2D` Stick_Axes))
        (:`>=`
          (`self.Compare to Dead Zone` (`KismetMathLibrary.BreakVector2D` Stick_Axes)
            (:`>=`
              (set `local.Stick_Dir_Temp` "NewEnumerator6"))
            (:`between`
              (set `local.Stick_Dir_Temp` "NewEnumerator0"))
            (:`<=`
              (set `local.Stick_Dir_Temp` "NewEnumerator9"))))
        (:`between`
          (`self.Compare to Dead Zone` (`KismetMathLibrary.BreakVector2D` Stick_Axes)
            (:`>=`
              (set `local.Stick_Dir_Temp` "NewEnumerator2"))
            (:`<=`
              (set `local.Stick_Dir_Temp` "NewEnumerator3"))))
        (:`<=`
          (`self.Compare to Dead Zone` (`KismetMathLibrary.BreakVector2D` Stick_Axes)
            (:`>=`
              (set `local.Stick_Dir_Temp` "NewEnumerator7"))
            (:`between`
              (set `local.Stick_Dir_Temp` "NewEnumerator1"))
            (:`<=`
              (set `local.Stick_Dir_Temp` "NewEnumerator8"))))))
    (:`then_1`
      (return (`local.Stick_Dir_Temp`)))))

(fn `CheckInputBufferForSpecial`
  (locals (Buffer_Index :type Integer) (whileBreak :type Boolean) (SpecialMoveValid :type Boolean :default false))
  (for _array_element (`/Game/Blueprints/Character/PDA_Chara.Specials` (`self.Chara_Data`))
    (set `local.Buffer_Index` (- (`KismetArrayLibrary.Array_Length` (`self.Input_Buffer`)) 1))
    (bind (_arrayindex _arrayelement) (`/Engine/EditorBlueprintResources/StandardMacros.ReverseForEachLoop` (`.Inputs_9_DAC3B6BC4849678E1B6387806B1EC4D9` (break `/Game/Blueprints/Character/F_info_Move` _array_element)))
      (:`LoopBody`
        (set `local.whileBreak` false)
        (while (and (>= (`local.Buffer_Index`) 0) (not (`local.whileBreak`)))
          (if (`self.Compare_BufferStruct_To_InputList` (`|GetArrayItem` (`self.Input_Buffer`) (`local.Buffer_Index`)) _arrayelement)
            (set `local.whileBreak` true)
            (else
              (`/Engine/EditorBlueprintResources/StandardMacros.DecrementInt` (`local.Buffer_Index`))))))
      (:`Completed`
        (if (>= (`local.Buffer_Index`) 0)
          (`self.PlaySpecialMove` _array_element)
          (break)))))
  (return))

(fn `Compare_BufferStruct_To_InputList`
  (params (Buffer_Entry :type "/Game/Blueprints/Character/Inputs/Struct_Buffer_Data Structure") (Input :type "/Game/Blueprints/Character/Inputs/E_Input_List Enum" :default "NewEnumerator8"))
  (returns (isEqual :type Boolean))
  (bind (_direction _punch _kick) (break `/Game/Blueprints/Character/Inputs/Struct_Buffer_Data` Buffer_Entry))
  (return (or (and (`|EnumEquality` Input "NewEnumerator4") _punch) (and (`|EnumEquality` Input "NewEnumerator5") _kick) (`|EnumEquality` _direction Input))))

(fn `Full Clean Input Buffer`
  (`KismetArrayLibrary.Array_Clear` (`self.Input_Buffer`)))

(fn `GetCurrentNormalData`
  (params (Normal :type "/Game/Blueprints/Character/E_Normal_Move Enum" :default "NewEnumerator1"))
  (returns (NormalMove :type "/Game/Blueprints/Character/F_info_Move Structure"))
  (locals (NormalTemp :type "/Game/Blueprints/Character/F_info_Move Structure"))
  (bind (_normals_punch_neutral _normals_punch_low _normals_punch_air _normals_kick_neutral _normals_kick_low _normals_kick_air) (break `/Game/Blueprints/Character/F_List_Normals` (`/Game/Blueprints/Character/PDA_Chara.Normals` (`self.Chara_Data`))))
  (`|ExecutionSequence`
    (:`then_0`
      (switch `/Game/Blueprints/Character/E_Normal_Move` Normal
        (:`NewEnumerator1`
          (set `local.NormalTemp` _normals_punch_neutral))
        (:`NewEnumerator6`
          (set `local.NormalTemp` _normals_punch_low))
        (:`NewEnumerator7`
          (set `local.NormalTemp` _normals_punch_air))
        (:`NewEnumerator2`
          (set `local.NormalTemp` _normals_kick_neutral))
        (:`NewEnumerator4`
          (set `local.NormalTemp` _normals_kick_low))
        (:`NewEnumerator5`
          (set `local.NormalTemp` _normals_kick_air))))
    (:`then_1`
      (return (`local.NormalTemp`)))))

(fn `GetCurrentSpecialData_FromName`
  (params (Name :type Name))
  (returns (SpecialMove :type "/Game/Blueprints/Character/F_info_Move Structure"))
  (for _array_element (`/Game/Blueprints/Character/PDA_Chara.Specials` (`self.Chara_Data`))
    (if (== (`.Move_Special_27_266779C148B0227E92249D8F15D0E583` (break `/Game/Blueprints/Character/F_info_Move` _array_element)) Name)
      (return _array_element))))

(fn `Record Input Buffer`
  (bind (_input_currentframe_direction _input_currentframe_punch _input_currentframe_kick) (break `/Game/Blueprints/Character/Inputs/Struct_Buffer_Data` (`self.Input_CurrentFrame`)))
  (bind _input_buffer (`self.Input_Buffer`))
  (`KismetArrayLibrary.Array_Add` _input_buffer (make `/Game/Blueprints/Character/Inputs/Struct_Buffer_Data` _input_currentframe_direction _input_currentframe_punch _input_currentframe_kick))
  (while (> (`KismetArrayLibrary.Array_Length` _input_buffer) 30)
    (`KismetArrayLibrary.Array_Remove` _input_buffer)))

(fn `UserConstructionScript`)